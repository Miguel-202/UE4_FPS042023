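; BP_WeaponBase is a base weapon Blueprint that fires projectiles on behalf of the pawn carrying it.
; On BeginPlay it caches its parent actor as the owning pawn, so it expects to be attached as a child actor.
; Shoot spawns the configured projectile class at the mesh's muzzle flash socket, rotated to the pawn's base aim rotation.
; The pawn's controller becomes the projectile's owner and the pawn its instigator.
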(event Custom|Shoot
  (bind _owningpawn (Variables|Default|GetOwningPawn))
  (Game|SpawnActorfromClass (Variables|Default|GetProjectileClass) (Math|Transform|MakeTransform (Transformation|GetSocketLocation (Variables|Default|GetSkeletalMesh) "MuzzleFlashSocket") (Pawn|GetBaseAimRotation _owningpawn) "1,1,1") "Undefined" (Pawn|GetController _owningpawn) _owningpawn))

(event EventBeginPlay
  (bind _aspawn (Utilities|Casting|CastToPawn (Actor|GetParentActor)))
  (Variables|Default|SetOwningPawn _aspawn))

(fn ConstructionScript)