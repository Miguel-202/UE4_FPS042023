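; BP_Player is the player Blueprint, handling look, movement and shooting input.
; Turn axes drive controller yaw and pitch, while move axes add movement along forward and right vectors built from control yaw only, so camera pitch does not affect direction.
; Pressing Shoot calls CharacterShoot, whose logic is not defined in these graphs; BeginPlay, overlap, Tick and construction add no custom logic.
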(event EventBeginPlay
  (|CallParentFunction) ; This node is disabled and will not be called.\nDrag off pins to build functionality.
)

(event Collision|EventActorBeginOverlap
  (params (OtherActor :type Actor%20Object%20Reference))
  (|CallParentFunction OtherActor) ; This node is disabled and will not be called.\nDrag off pins to build functionality.
)

(event EventTick
  (params (DeltaSeconds :type Float%20%28single-precision%29))
  (|CallParentFunction DeltaSeconds) ; This node is disabled and will not be called.\nDrag off pins to build functionality.
)

(event Input|ActionEvents|InputActionShoot
  (params (Key :type Key%20Structure :default "None"))
  (:Pressed
    (CallFunction|CharacterShoot)))

(event Input|AxisEvents|InputAxisTurnHorizontal
  (params (AxisValue :type Float%20%28single-precision%29))
  ;[1 1 1] Rotation
  (Pawn|Input|AddControllerYawInput AxisValue))

(event Input|AxisEvents|InputAxisTurnVertical
  (params (AxisValue :type Float%20%28single-precision%29))
  ;[1 1 1] Rotation
  (Pawn|Input|AddControllerPitchInput AxisValue))

(event Input|AxisEvents|InputAxisMoveForward
  (params (AxisValue :type Float%20%28single-precision%29))
  ;[1 1 1] Player Movement
  (Pawn|Input|AddMovementInput (Math|Vector|GetForwardVector (Math|Rotator|MakeRotator 0.0 0.0 (.yaw (Pawn|GetControlRotation :!class /Script/Engine.Pawn)))) AxisValue false))

(event Input|AxisEvents|InputAxisMoveRight
  (params (AxisValue :type Float%20%28single-precision%29))
  ;[1 1 1] Player Movement
  (Pawn|Input|AddMovementInput (Math|Vector|GetRightVector (Math|Rotator|MakeRotator 0.0 0.0 (.yaw (Pawn|GetControlRotation :!class /Script/Engine.Pawn)))) AxisValue false))

(fn ConstructionScript
  (|CallParentFunction))