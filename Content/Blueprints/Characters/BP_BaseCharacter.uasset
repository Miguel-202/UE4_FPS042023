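; BP_BaseCharacter is a base character Blueprint that equips a weapon and provides a shoot event.
; On BeginPlay it spawns WeaponClass through the WeaponChild child actor component and caches it as a BP_WeaponBase.
; It then caches the mesh's ABP_Riffle anim instance and binds to the weapon's OnShoot, printing a message if either cast fails.
; CharacterShoot forwards firing to the current weapon.
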(event Custom|CharacterShoot
  (Default|Shoot (Variables|Default|GetCurrentWeapon)))

(event EventBeginPlay
  (bind _weaponchild (Variables|Default|GetWeaponChild))
  (ChildActorComponent|SetChildActorClass _weaponchild (Variables|Default|GetWeaponClass))
  (bind _asbp_weapon_base (Utilities|Casting|CastToBP_WeaponBase (Variables|/Script/Engine.ChildActorComponent|GetChildActor _weaponchild))
    (:then
      (Variables|Default|SetCurrentWeapon _asbp_weapon_base)
      (bind _asabp_riffle (Utilities|Casting|CastToABP_Riffle (Components|SkeletalMesh|GetAnimInstance (Variables|Character|GetMesh)))
        (:then
          (Variables|Default|SetAnimationBP _asabp_riffle)
          (EventDispatchers|BindEventtoOnShoot (Variables|Default|GetCurrentWeapon) (EventDispatchers|CreateEvent (Variables|Default|GetAnimationBP) :!event PlayShootAnimation)))
        (:CastFailed
          (Development|PrintString "Bad Animation class"))))
    (:CastFailed
      (Development|PrintString "No weapon to use"))))

(fn ConstructionScript)