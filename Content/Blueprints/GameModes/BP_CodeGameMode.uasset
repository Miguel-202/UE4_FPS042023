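; BP_CodeGameMode is a game mode Blueprint that ends the match in a win once the enemies are destroyed.
; On BeginPlay it counts all BaseAI actors and binds their OnDestroyed events to EnemyDies, which decrements the count.
; When the count hits zero, it shows WBP_Results with win results for the player controller, then a timer has END_GameInstance load the main menu.
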(event Custom|EnemyDies
  (params (DestroyedActor :type Actor%20Object%20Reference))
  (if (Utilities|IsValid DestroyedActor)
    (bind _result (Math|Integer|DecrementInt (Variables|Default|GetEnemiesCount))
      (:%20%20
        (if (== 0 _result)
          (bind _returnvalue (Actor|GetActorOfClass (Variables|Default|GetPlayerControllerClass)))
          (bind _output_get (Variables|Default|SetCurrentPC _returnvalue))
          (bind _returnvalue_2 (UserInterface|CreateWidget "/Game/Widgets/WBP_Results.WBP_Results_C" _output_get))
          (bind _output_get_2 (Variables|Default|SetResultsScreen _returnvalue_2))
          (UserInterface|Viewport|AddtoViewport _output_get_2 0)
          (Class|ResultsWidget|SetWinResults _output_get_2)
          (Utilities|Time|SetTimerbyEvent (delegate Custom|LoadMainMenu) 5.0))))))

(event Custom|LoadMainMenu
  (bind _asend_game_instance (Utilities|Casting|CastToEND_GameInstance (Game|GetGameInstance)))
  (Class|ENDGameInstance|LoadMainMenu _asend_game_instance))

(event EventBeginPlay
  (bind _outactors (Actor|GetAllActorsOfClass "/Script/FPS042023.BaseAI"))
  (Variables|Default|SetEnemiesCount (Utilities|Array|Length _outactors))
  (for _array_element _outactors
    (Game|BindEventtoOnDestroyed _array_element (delegate Custom|EnemyDies))))

(event EventTick
  (params (DeltaSeconds :type Float%20%28single-precision%29)))

(fn ConstructionScript)